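; Parent paddle Blueprint, apparently for a Pong-style game, that keeps its Cube within a vertical range.
; Tick calls a local offset with no delta set, then limits the Cube's world Z through ClampVectorSize, leaving X and Y unchanged.
; A PaddleWrap function, not called here, offsets the Cube opposite its Z beyond a wider threshold, scaled by a per-side multiplier.
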(event `self.ReceiveBeginPlay`)

(event `self.ReceiveActorBeginOverlap`
  (params (OtherActor :type "Actor Object Reference")))

(event `self.ReceiveTick`
  (params (DeltaSeconds :type "Float (single-precision)"))
  (bind _cube (`self.Cube`))
  (bind (_returnvalue_x _returnvalue_y _returnvalue_z) (`KismetMathLibrary.BreakVector` (`SceneComponent.K2_GetComponentLocation` _cube)))
  (bind (_returnvalue_x_2 _returnvalue_y_2) (`KismetMathLibrary.BreakVector` (`SceneComponent.K2_GetComponentLocation` _cube)))
  (bind (_returnvalue_x_3 _returnvalue_y_3 _returnvalue_z_2) (`KismetMathLibrary.BreakVector` (`KismetMathLibrary.ClampVectorSize` (`KismetMathLibrary.MakeVector` 0.0 0.0 _returnvalue_z) -345.0 345.0)))
  (`SceneComponent.K2_AddLocalOffset` _cube (0.0 0.0 0.0) false false)
  (`SceneComponent.K2_SetWorldLocation` (`self.Cube`) (`KismetMathLibrary.MakeVector` _returnvalue_x_2 _returnvalue_y_2 _returnvalue_z_2) false false))

(fn `PaddleWrap`
  (params (C :type "Float (double-precision)") (C2 :type "Float (double-precision)"))
  (bind _cube (`self.Cube`))
  (bind _cube_2 (`self.Cube`))
  (bind (_returnvalue_x _returnvalue_y _returnvalue_z) (`KismetMathLibrary.BreakVector` (`SceneComponent.K2_GetComponentLocation` _cube)))
  (bind (_returnvalue_x_2 _returnvalue_y_2 _returnvalue_z_2) (`KismetMathLibrary.BreakVector` (`SceneComponent.K2_GetComponentLocation` _cube_2)))
  (bind (_returnvalue_x_3 _returnvalue_y_3 _returnvalue_z_3) (`KismetMathLibrary.BreakVector` (`SceneComponent.K2_GetComponentLocation` (`self.Cube`))))
  (if (>= _returnvalue_z_3 400.0)
    (bind _output_get (set `self.Cube` _cube_2))
    (`SceneComponent.K2_AddLocalOffset` _output_get (`KismetMathLibrary.MakeVector` 0.0 0.0 (* _returnvalue_z_2 -120.0 C)) false false)
    (elif (<= _returnvalue_z_3 -400.0)
      (bind _output_get_2 (set `self.Cube` _cube))
      (`SceneComponent.K2_AddLocalOffset` _output_get_2 (`KismetMathLibrary.MakeVector` 0.0 0.0 (* _returnvalue_z -120.0 C2)) false false))))

(fn `UserConstructionScript`)